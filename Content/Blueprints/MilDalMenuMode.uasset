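; MilDalMenuMode manages endless-style floor building, respawns and lives for a two-player game.
; AddFloorTile spawns a random tile class at NextSpawnPoint, then takes the next point from that tile's attach transform.
; RespawnPlayer repositions players relative to the main camera with clamped Y, then calls their respawn-ready function.
; Life changes pick the player by tag and update UI icons, with losses ignored after game over.
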(fn ConstructionScript)

(fn AddFloorTile
  (bind _floortiles (Variables|Default|GetFloorTiles))
  ;[1 1 1] 맵을 추가하는 함수
  (bind _returnvalue (Game|SpawnActorfromClass (Utilities|Array|Get(acopy) _floortiles (Math|Random|RandomIntegerinRange 0 (Utilities|Array|LastIndex _floortiles))) (Variables|Default|GetNextSpawnPoint) "Undefined" 0 0))
  (bind _asbp_floor_tile_basic (Utilities|Casting|CastToBP_FloorTileBasic _returnvalue))
  (bind _attachtransform (Default|GetAttachTransform _asbp_floor_tile_basic))
  (Variables|Default|SetNextSpawnPoint _attachtransform))

(fn RespawnPlayer
  (params (Player :type Actor%20Object%20Reference))
  (bind _maincamera (Variables|Default|GetMainCamera))
  (bind _returnvalue (Transformation|GetActorLocation _maincamera))
  (bind (_x _y _z) (Math|Vector|BreakVector _returnvalue))
  ;[1 1 1] 플레이어 리스폰
  (Transformation|SetActorLocation Player (Math|Vector|MakeVector (+ _x 6e+02) (Math|Float|Clamp(Float) (.Y (Math|Vector|BreakVector (Transformation|GetActorLocation Player))) -4.5e+02 4.5e+02) (+ _z -3e+02)) false false)
  (if (Actor|ActorHasTag Player "Player1P")
    (bind _asbp_player_1p (Utilities|Casting|CastToBP_Player1P Player))
    (Default|RespawnReady1P _asbp_player_1p)
    (else
      (bind _asbp_player_2p (Utilities|Casting|CastToBP_Player2P Player))
      (Default|RespawnReady2P _asbp_player_2p))))

(fn ReduceLife
  (params (Player :type Actor%20Object%20Reference))
  (bind _uiblueprint (Variables|Default|GetUIBluePrint))
  ;[1 1 1] 목숨 감소
  (if (not (Variables|Default|GetGameOver))
    (if (Actor|ActorHasTag Player "Player1P")
      (bind _output_get (Variables|Default|SetPlayer1PLife (- (Variables|Default|GetPlayer1PLife) 1)))
      (Default|UIReduceLifeIcon _uiblueprint true _output_get)
      (else
        (bind _output_get_2 (Variables|Default|SetPlayer2PLife (- (Variables|Default|GetPlayer2PLife) 1)))
        (Default|UIReduceLifeIcon _uiblueprint false _output_get_2)))))

(fn IncreaseLife
  (params (Player :type Actor%20Object%20Reference))
  (bind _uiblueprint (Variables|Default|GetUIBluePrint))
  ;[1 1 1] 목숨 증가
  (if (Actor|ActorHasTag Player "Player1P")
    (bind _output_get (Variables|Default|SetPlayer1PLife (+ (Variables|Default|GetPlayer1PLife) 1)))
    (Default|UIIncreaseLifeIcon _uiblueprint true _output_get)
    (else
      (bind _output_get_2 (Variables|Default|SetPlayer2PLife (+ (Variables|Default|GetPlayer2PLife) 1)))
      (Default|UIIncreaseLifeIcon _uiblueprint false _output_get_2))))