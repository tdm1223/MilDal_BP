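; MilDalGameMode runs a two-player falling match with lives, respawns and win checks.
; BeginPlay caches both players and the main camera by tag; Tick respawns anyone below DropHeight relative to the camera.
; Drops call ReduceLife without a Player argument; zero lives prints the opponent's win and calls SetGamePaused(false), so nothing pauses.
; AddFloorTile, uncalled here, chains random tiles via each tile's attach transform.
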(event Custom|Player1P%20Win
  ;[1 1 1] 플레이어의 승리로 게임 종료
  (Game|SetGamePaused false) ; Pause를 True로
  (Development|PrintString "1P 승리!"))

(event Custom|Player1P%20Drop
  ;[1 1 1] 플레이어들이 떨어졌을 때 실행되는 이벤트
  (CallFunction|RespawnPlayer (Variables|Default|GetPlayer1P))
  (CallFunction|ReduceLife)
  ;[1 1 1] 목숨이 0 이하면 상대방의 승리 이벤트 수행
  (if (<= (Variables|Default|GetPlayer1PLife) 0)
    (CallFunction|Player2PWin)))

(event Custom|Player2P%20Win
  ;[1 1 1] 플레이어의 승리로 게임 종료
  (Game|SetGamePaused false)
  (Development|PrintString "2P 승리!"))

(event Custom|Player2P%20Drop
  ;[1 1 1] 플레이어들이 떨어졌을 때 실행되는 이벤트
  (CallFunction|RespawnPlayer (Variables|Default|GetPlayer2P))
  (CallFunction|ReduceLife)
  ;[1 1 1] 목숨이 0 이하면 상대방의 승리 이벤트 수행
  (if (<= (Variables|Default|GetPlayer2PLife) 0)
    (CallFunction|Player1PWin)))

(event EventTick
  (params (DeltaSeconds :type Float%20%28single-precision%29))
  ;[1 1 1] 매 초마다 떨어지는 높이 이하인치 판단하여 Player Drop 이벤트 수행
  (Utilities|FlowControl|Sequence
    (:then_0
      (if (<= (.Z (Math|Vector|BreakVector (Transformation|GetActorLocation (Variables|Default|GetPlayer1P)))) (Variables|Default|GetDropHeight))
        (CallFunction|Player1PDrop)))
    (:then_1
      (if (<= (.Z (Math|Vector|BreakVector (Transformation|GetActorLocation (Variables|Default|GetPlayer2P)))) (Variables|Default|GetDropHeight))
        (CallFunction|Player2PDrop)))))

(event EventBeginPlay
  ;[1 1 1] 플레이어와 카메라 초기화
  (Utilities|FlowControl|Sequence
    (:then_0
      (bind _outactors (Actor|GetAllActorswithTag "Player"))
      (for _array_element _outactors
        (if (Actor|ActorHasTag _array_element "Player1P")
          (bind _asbp_player_1p (Utilities|Casting|CastToBP_Player1P _array_element))
          (Variables|Default|SetPlayer1P _asbp_player_1p)
          (else
            (bind _asbp_player_2p (Utilities|Casting|CastToBP_Player2P _array_element))
            (Variables|Default|SetPlayer2P _asbp_player_2p)))))
    (:then_1
      (bind _outactors_2 (Actor|GetAllActorswithTag "MainCamera"))
      (for _array_element_2 _outactors_2
        (bind _asbp_main_camera (Utilities|Casting|CastToBP_MainCamera _array_element_2))
        (Variables|Default|SetMainCamera _asbp_main_camera)))))

(fn ConstructionScript)

(fn AddFloorTile
  (params (NewParam :type Boolean))
  (bind _floortiles (Variables|Default|GetFloorTiles))
  ;[1 1 1] 맵을 추가하는 함수
  (bind _returnvalue (Game|SpawnActorfromClass (Utilities|Array|Get(acopy) _floortiles (Math|Random|RandomIntegerinRange 0 (Utilities|Array|LastIndex _floortiles))) (Variables|Default|GetNextSpawnPoint) "Undefined" 0 0))
  (bind _asbp_floor_tile_basic (Utilities|Casting|CastToBP_FloorTileBasic _returnvalue))
  (bind _attachtransform (Default|GetAttachTransform _asbp_floor_tile_basic))
  (Variables|Default|SetNextSpawnPoint _attachtransform))

(fn RespawnPlayer
  (params (Player :type Actor%20Object%20Reference))
  (bind _maincamera (Variables|Default|GetMainCamera))
  (bind _returnvalue (Transformation|GetActorLocation _maincamera))
  (bind (_x _y _z) (Math|Vector|BreakVector _returnvalue))
  ;[1 1 1] 플레이어 리스폰
  (Transformation|SetActorLocation Player (Math|Vector|MakeVector (+ _x 6e+02) (Math|Float|Clamp(Float) (.Y (Math|Vector|BreakVector (Transformation|GetActorLocation Player))) -4.5e+02 4.5e+02) (+ _z -3e+02)) false false)
  (if (Actor|ActorHasTag Player "Player1P")
    (bind _asbp_player_1p (Utilities|Casting|CastToBP_Player1P Player))
    (Default|RespawnReady1P _asbp_player_1p)
    (else
      (bind _asbp_player_2p (Utilities|Casting|CastToBP_Player2P Player))
      (Default|RespawnReady2P _asbp_player_2p))))

(fn ReduceLife
  (params (Player :type Actor%20Object%20Reference))
  ;[1 1 1] 목숨 감소
  (if (Actor|ActorHasTag Player "Player1P")
    (Variables|Default|SetPlayer1PLife (- (Variables|Default|GetPlayer1PLife) 1))
    (else
      (Variables|Default|SetPlayer2PLife (- (Variables|Default|GetPlayer2PLife) 1)))))