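; Arena background actor (배경BP) that scrolls its background component along X during gameplay.
; While IsGamePlay is set, Tick adds a world offset of 배경이동속도 each frame, without sweep or delta-time scaling, so scroll speed depends on frame rate.
; After each move it checks GameOver on ThirdPersonGameMode and zeroes the speed to stop the scroll when the game ends.
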(event EventTick
  (params (DeltaSeconds :type Float%20%28single-precision%29))
  ;[1 1 1] 배경이동
  (if (Variables|Default|GetisGamePlay)
    (Transformation|AddWorldOffset (Variables|Default|Get배경) (Math|Vector|MakeVector (Variables|Default|Get배경이동속도) 0.0 0.0) false false)
    ;;[1 1 1] 0606이후 추가 게임이끝나면 더이상 움직이지 않음
    (bind _asthird_person_game_mode (Utilities|Casting|CastToThirdPersonGameMode (Game|GetGameMode)))
    (if (Variables|/Game/Blueprints/Player/ThirdPersonGameMode.ThirdPersonGameMode_C|GetGameOver _asthird_person_game_mode)
      (Variables|Default|Set배경이동속도 0.0))))

(fn ConstructionScript)