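; BP_FloorTileBasic is a floor tile for an endlessly extending track, exposing an attach transform where the next tile connects.
; On BeginPlay it makes repeated weighted random rolls to spawn at most one random item inside ItemArena, attached to the tile.
; When MainCamera_Blueprint overlaps EndTrigger, it asks ThirdPersonGameMode for another tile, then destroys itself and its item after a delay, or immediately on game over.
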(event OnComponentBeginOverlap(EndTrigger)
  (params (OverlappedComponent :type Primitive%20Component%20Object%20Reference) (OtherActor :type Actor%20Object%20Reference) (OtherComp :type Primitive%20Component%20Object%20Reference) (OtherBodyIndex :type Integer) (bFromSweep :type Boolean) (SweepResult :type Hit%20Result%20Structure%20%28by%20ref%29))
  ;[1 1 1] 맵끝부분에 닿으면 다음 타일 생성후 이전타일삭제
  (Utilities|Casting|CastToMainCamera_Blueprint OtherActor)
  (bind _asthird_person_game_mode (Utilities|Casting|CastToThirdPersonGameMode (Game|GetGameMode)))
  (if (Variables|/Game/Blueprints/ThirdPersonGameMode.ThirdPersonGameMode_C|GetGameOver _asthird_person_game_mode)
    (Actor|DestroyActor)
    (Actor|DestroyActor (stale EventBeginPlay _item))
    (else
      (Default|AddFloorTile _asthird_person_game_mode)
      (Utilities|FlowControl|Delay 2.0)
      (Actor|DestroyActor)
      (Actor|DestroyActor (stale EventBeginPlay _item)))))

(event EventBeginPlay
  ;[1 1 1] 아이템생성
  (bind _item (CallFunction|아이템생성)))

(fn ConstructionScript
  ;[1 1 1] 아이템 배열 세팅
  (Variables|Default|Set아이템배열 (Utilities|Array|MakeArray "/Game/Blueprints/Item/Fast.Fast_C" "/Game/Blueprints/Item/InfiniteJump.InfiniteJump_C" "/Game/Blueprints/Item/Reverse.Reverse_C" "/Game/Blueprints/Item/Push.Push_C" "/Game/Blueprints/Item/Heart.Heart_C")))

(fn GetAttachTransform
  ;[1 1 1] 다음 맵이 붙는 장소 반환하는 함수
  (return (Transformation|GetWorldTransform (Variables|Default|GetAttachPoint))))

(fn 아이템생성
  (bind _itemarena (Variables|Default|GetItemArena))
  ;[1 1 1] 아이템 아레나의 랜덤범위 안에서 주어진 아이템 배열중 하나를 랜덤으로 선택하여 스폰하는 함수
  (for _index (range 0 10)
    (if (<= (* (Math|Random|RandomFloatinRange 0.0 5e+02) (Variables|Default|Get아이템확률)) 1e+02)
      (bind _returnvalue (Game|SpawnActorfromClass (Utilities|Array|Get(acopy) (Variables|Default|Get아이템배열) (Math|Random|RandomIntegerinRange 0 4)) (Math|Conversions|ToTransform(Vector) (Math|Random|RandomPointinBoundingBox (Variables|/Script/Engine.SceneComponent|GetRelativeLocation _itemarena) (Variables|/Script/Engine.BoxComponent|GetBoxExtent _itemarena))) "Undefined" 0 0))
      (Transformation|AttachActorToActor _returnvalue self "None" "KeepRelative" "KeepRelative" "KeepRelative" true)
      (return _returnvalue))))