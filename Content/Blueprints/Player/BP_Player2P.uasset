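; Player 2 character for a two-player game, with item effects, a respawn pause and a shove against Player 1.
; Item events temporarily toggle Reverse, Fast or InfiniteJump (also raising the jump count), or spawn a Wind actor.
; Respawn zeroes gravity and velocity, blinking the mesh in a delay loop that ends when gravity is restored.
; PushCollision overlaps launch Player 1 away while this character is grounded; the construction script sets movement tuning.
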(event OnComponentBeginOverlap(PushCollision)
  (params (OverlappedComponent :type Primitive%20Component%20Object%20Reference) (OtherActor :type Actor%20Object%20Reference) (OtherComp :type Primitive%20Component%20Object%20Reference) (OtherBodyIndex :type Integer) (bFromSweep :type Boolean) (SweepResult :type Hit%20Result%20Structure%20%28by%20ref%29))
  ;[1 1 1] 미는 범위 안에 상대방이 들어왔는지 체크
  (if (and (Actor|ActorHasTag OtherActor "Player1P") (AI|Components|NavMovement|IsMovingonGround (Variables|Character|GetCharacterMovement)))
    (bind _asplayer_1p (Utilities|Casting|CastToBP_Player1P OtherActor))
    (Physics|AddImpulse (Variables|/Script/Engine.Character|GetCharacterMovement _asplayer_1p) (Math|Vector|MakeVector (.X (Math|Vector|BreakVector (* (- (Transformation|GetWorldLocation (Variables|/Script/Engine.Character|GetCapsuleComponent _asplayer_1p)) (Transformation|GetWorldLocation (Variables|Collision|GetCapsuleComponent))) (Variables|Default|Get미는힘)))) (.Y (Math|Vector|BreakVector (* (- (Transformation|GetWorldLocation (Variables|/Script/Engine.Character|GetCapsuleComponent _asplayer_1p)) (Transformation|GetWorldLocation (Variables|Collision|GetCapsuleComponent))) (Variables|Default|Get미는힘)))) 1e+02) true)))

(event Custom|MakeWind
  ;[1 1 1] 바람 아이템 생성
  (Game|SpawnActorfromClass "/Game/Blueprints/Item/WInd.WInd_C" (Transformation|GetActorTransform) "Undefined" 0 0))

(event Custom|setReverse2P
  ;[1 1 1] 반대 아이템
  (Variables|Default|SetReverse (not (Variables|Default|GetReverse)))
  (Utilities|FlowControl|Delay 5.0)
  (Variables|Default|SetReverse (not (Variables|Default|GetReverse))))

(event Custom|setFast2P
  ;[1 1 1] 선풍기 아이템
  (Variables|Default|SetFast (not (Variables|Default|GetFast)))
  (Utilities|FlowControl|Delay 1.0)
  (Variables|Default|SetFast (not (Variables|Default|GetFast))))

(event Custom|RespawnReady2P
  (bind _mesh (Variables|Character|GetMesh))
  (bind _charactermovement (Variables|Character|GetCharacterMovement))
  ;[1 1 1] 리스폰을 2초동안 대기하고 깜빡거림
  (Variables|/Script/Engine.CharacterMovementComponent|SetGravityScale _charactermovement 0.0)
  (Variables|/Script/Engine.MovementComponent|SetVelocity _charactermovement "0, 0, 0")
  (Utilities|FlowControl|Sequence
    (:then_0
      (Utilities|FlowControl|Delay 2.0)
      (Variables|/Script/Engine.CharacterMovementComponent|SetGravityScale _charactermovement 2.0))
    (:then_1
      (if (!= (Variables|/Script/Engine.CharacterMovementComponent|GetGravityScale _charactermovement) 2.0) :!label _label
        (Utilities|FlowControl|Delay 0.1)
        (Rendering|SetVisibility _mesh (not (Variables|Default|GetBlinkVisibility)) false)
        (Variables|Default|SetBlinkVisibility (not (Variables|Default|GetBlinkVisibility)))
        (goto _label)
        (else
          (bind _output_get (Variables|Default|SetBlinkVisibility true))
          (Rendering|SetVisibility _mesh _output_get false))))))

(event Custom|setInfiniteJump2P
  ;[1 1 1] 무한점프 아이템
  (Variables|Default|SetInfiniteJump (not (Variables|Default|GetInfiniteJump)))
  (Variables|Default|SetJumpMaxCount 100)
  (Utilities|FlowControl|Delay 5.0)
  (Variables|Default|SetInfiniteJump (not (Variables|Default|GetInfiniteJump)))
  (Variables|Default|SetJumpMaxCount 1))

(fn ConstructionScript
  (bind _charactermovement (Variables|Character|GetCharacterMovement))
  ;[1 1 1] 캐릭터 최대 속도 세팅
  (Variables|/Script/Engine.CharacterMovementComponent|SetMaxWalkSpeed _charactermovement 1e+03)
  (Variables|/Script/Engine.CharacterMovementComponent|SetAirControl _charactermovement 1.0)
  (Variables|/Script/Engine.CharacterMovementComponent|SetJumpZVelocity _charactermovement 1.3e+03)
  (Variables|/Script/Engine.CharacterMovementComponent|SetGravityScale _charactermovement 2.0))