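; Main camera actor for a two-player auto-scrolling game that drops players who fall behind it.
; While IsGamePlay is set, Tick moves its scene component along world X by a speed variable, without scaling by delta time.
; OutTrigger, behind the camera, catches overlapping Player-tagged actors and calls Player1PDrop or Player2PDrop on ThirdPersonGameMode, depending on the Player1P tag.
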(event OnComponentBeginOverlap(OutTrigger)
  (params (OverlappedComponent :type Primitive%20Component%20Object%20Reference) (OtherActor :type Actor%20Object%20Reference) (OtherComp :type Primitive%20Component%20Object%20Reference) (OtherBodyIndex :type Integer) (bFromSweep :type Boolean) (SweepResult :type Hit%20Result%20Structure%20%28by%20ref%29))
  ;[1 1 1] 카메라의 뒷쪽으로 플레이어가 벗어났을 때 PlayerDrop 처리
  (if (Actor|ActorHasTag OtherActor "Player")
    (bind _asthird_person_game_mode (Utilities|Casting|CastToThirdPersonGameMode (Game|GetGameMode)))
    (if (Actor|ActorHasTag OtherActor "Player1P")
      (Default|Player1PDrop _asthird_person_game_mode)
      (else
        (Default|Player2PDrop _asthird_person_game_mode)))))

(event EventTick
  (params (DeltaSeconds :type Float%20%28single-precision%29))
  ;[1 1 1] 게임 플레이 시 카메라 자동 움직임
  (if (Variables|Default|GetisGamePlay)
    (Transformation|AddWorldOffset (Variables|Default|GetSceneComponent) (Math|Vector|MakeVector (Variables|Default|Get카메라이동속도) 0.0 0.0) false false)))

(fn ConstructionScript)