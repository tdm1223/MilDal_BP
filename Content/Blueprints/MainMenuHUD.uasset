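; Main menu HUD that shows the menu widget and cycles background videos behind it.
; BeginPlay creates the menu widget and adds it to the viewport.
; Tick uses a flag and a delay as a timer loop, opening and playing a randomly picked source from the first two array entries on the BGVideo player every few seconds.
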(event EventBeginPlay
  ;[1 1 1] 시작시 위젯 생성하여 뷰포트에 추가
  (bind _returnvalue (UserInterface|CreateWidget "/Game/Blueprints/MenuWidget.MenuWidget_C"))
  (UserInterface|Viewport|AddtoViewport _returnvalue 0))

(event EventTick
  (params (DeltaSeconds :type Float%20%28single-precision%29))
  (bind _bgvideo (Variables|Default|GetBGVideo))
  ;[1 1 1] 배경 비디오 재생
  (if (Variables|Default|GetPlayFlag)
    (Media|MediaPlayer|OpenSource _bgvideo (Utilities|Array|Get(acopy) (Variables|Default|GetBGArray) (Math|Random|RandomInteger 2)))
    (Media|MediaPlayer|Play _bgvideo :!class /Script/MediaAssets.MediaPlayer)
    (Variables|Default|SetPlayFlag false)
    (Utilities|FlowControl|Delay 7.0)
    (Variables|Default|SetPlayFlag true)))

(fn ConstructionScript)