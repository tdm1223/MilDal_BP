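; BP_FloorTileBasic is a floor tile that keeps the level extending as the main camera advances.
; When MainCamera_Blueprint overlaps EndTrigger, it asks ThirdPersonGameMode to add the next tile, then destroys itself after a short delay.
; GetAttachTransform exposes the AttachPoint world transform.
; The OutTrigger overlap does nothing, as its player respawn logic is disconnected.
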(event OnComponentBeginOverlap(EndTrigger)
  (params (OverlappedComponent :type Primitive%20Component%20Object%20Reference) (OtherActor :type Actor%20Object%20Reference) (OtherComp :type Primitive%20Component%20Object%20Reference) (OtherBodyIndex :type Integer) (bFromSweep :type Boolean) (SweepResult :type Hit%20Result%20Structure%20%28by%20ref%29))
  ;[1 1 1] 맵끝부분에 닿으면 다음 타일 생성후 이전타일삭제
  (Utilities|Casting|CastToMainCamera_Blueprint OtherActor)
  (bind _asthird_person_game_mode (Utilities|Casting|CastToThirdPersonGameMode (Game|GetGameMode)))
  (Default|AddFloorTile _asthird_person_game_mode false)
  (Utilities|FlowControl|Delay 2.0)
  (Actor|DestroyActor))

(event OnComponentBeginOverlap(OutTrigger)
  (params (OverlappedComponent :type Primitive%20Component%20Object%20Reference) (OtherActor :type Actor%20Object%20Reference) (OtherComp :type Primitive%20Component%20Object%20Reference) (OtherBodyIndex :type Integer) (bFromSweep :type Boolean) (SweepResult :type Hit%20Result%20Structure%20%28by%20ref%29))
  ;[1 1 1] 바닥에 떨어지면 캐릭터 부활
)

(fn ConstructionScript)

(fn GetAttachTransform
  (return (Transformation|GetWorldTransform (Variables|Default|GetAttachPoint))))