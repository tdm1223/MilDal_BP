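; World-space UI actor for a two-player game, showing ready text, countdown, lives and winner.
; BeginPlay spawns a row of mesh life icons per player from ThirdPersonGameMode's life counts; events hide or reveal them by index.
; The countdown chains Timelines that pulse 3, 2, 1 and start text, playing a sound at start.
; On a win, MoveComponentTo slides in the winner text, then a clickable restart text appears that reloads the level.
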(event OnClicked(TextRestartButton)
  (params (TouchedComponent :type Primitive%20Component%20Object%20Reference) (ButtonPressed :type Key%20Structure :default "AnyKey"))
  (bind _returnvalue (Game|GetCurrentLevelName true))
  (Game|OpenLevel(byName) (Utilities|String|StringToName _returnvalue))
  (Development|PrintString "Hello"))

(event Custom|UIPlayerWin
  (params (isPlayer1P :type Boolean))
  (bind _textrestartbutton (Variables|Default|GetTextRestartButton))
  ;[1 1 1] 게임오버가 되면 승자 텍스트를 내리고 다시시작 버튼을 보이게 함
  (if isPlayer1P
    (Components|MoveComponentTo (Variables|Default|GetTextPlayer1PWin) "80.000000,0.000000,-40.000000" "0,180.000000, 0" true false 0.5 false)
    (else
      (Components|MoveComponentTo (Variables|Default|GetTextPlayer2PWin) "80.000000,0.000000,-40.000000" "0,180.000000, 0" true false 0.5 false)))
  (Utilities|FlowControl|Delay 0.5)
  (Rendering|SetVisibility _textrestartbutton true false)
  (Collision|SetCollisionResponsetoAllChannels _textrestartbutton "ECR_Block"))

(event Custom|UIReduceLifeIcon
  (params (isPlayer1P :type Boolean) (PlayerLife :type Integer))
  ;[1 1 1] 생명력이 깎일 때 아이콘을 보이지 않도록
  (if isPlayer1P
    (Rendering|SetVisibility (Utilities|Array|Get(acopy) (Variables|Default|GetPlayer1PLifeIconArr) PlayerLife) false false)
    (else
      (Rendering|SetVisibility (Utilities|Array|Get(acopy) (Variables|Default|GetPlayer2PLifeIconArr) PlayerLife) false false))))

(event Custom|UIIncreaseLifeIcon
  (params (IsPlayer1P :type Boolean) (PlayerLife :type Integer))
  (bind _returnvalue (- PlayerLife 1))
  ;[1 1 1] 생명력이 추가될때 아이콘이 보이도록
  (if IsPlayer1P
    (Rendering|SetVisibility (Utilities|Array|Get(acopy) (Variables|Default|GetPlayer1PLifeIconArr) _returnvalue) true false)
    (else
      (Rendering|SetVisibility (Utilities|Array|Get(acopy) (Variables|Default|GetPlayer2PLifeIconArr) _returnvalue) true false))))

(event Custom|UICountDown
  ;[1 1 1] 플레이어들의 READY 텍스트를 끄고 3초간 카운트 다운
  (Rendering|SetVisibility (Variables|Default|GetTextJumpToReady) false false)
  (Rendering|SetVisibility (Variables|Default|GetTextCount3) true false)
  (bind _pulsemovement (Timeline|CountDownNumber3Anim Play)
    (:Update
      (Transformation|SetRelativeScale3D (Variables|Default|GetTextCount3) (Math|Vector|Lerp(Vector) "1.000000,1.000000,1.000000" "3.000000,3.000000,3.000000" _pulsemovement)))
    (:Finished
      (Rendering|SetVisibility (Variables|Default|GetTextCount3) false false)
      (Rendering|SetVisibility (Variables|Default|GetTextCount2) true false)
      (bind _pulsemovement_2 (Timeline|CountDownNumber2Anim Play)
        (:Update
          (Transformation|SetRelativeScale3D (Variables|Default|GetTextCount2) (Math|Vector|Lerp(Vector) "1.000000,1.000000,1.000000" "3.000000,3.000000,3.000000" _pulsemovement_2)))
        (:Finished
          (Rendering|SetVisibility (Variables|Default|GetTextCount2) false false)
          (Rendering|SetVisibility (Variables|Default|GetTextCount1) true false)
          (bind _pulsemovement_3 (Timeline|CountDownNumber1Anim Play)
            (:Update
              (Transformation|SetRelativeScale3D (Variables|Default|GetTextCount1) (Math|Vector|Lerp(Vector) "1.000000,1.000000,1.000000" "3.000000,3.000000,3.000000" _pulsemovement_3))
              (Rendering|SetVisibility (Variables|Default|GetTextPlayer1PReady) false false)
              (Rendering|SetVisibility (Variables|Default|GetTextPlayer2PReady) false false))
            (:Finished
              (Rendering|SetVisibility (Variables|Default|GetTextCount1) false false)
              (Rendering|SetVisibility (Variables|Default|GetTextStrat) true false)
              (Audio|PlaySoundatLocation "/Game/StaticMesh/Sound/기타음악소스/SoundGamePlay.SoundGamePlay" "0, 0, 0" "0, 0, 0" 2.5 1.0 0.5)
              (bind _pulsemovement_4 (Timeline|CountDownStartAnim Play)
                (:Update
                  (Transformation|SetRelativeScale3D (Variables|Default|GetTextStrat) (Math|Vector|Lerp(Vector) "1.000000,1.000000,1.000000" "1.500000,1.500000,1.500000" _pulsemovement_4)))
                (:Finished
                  (Rendering|SetVisibility (Variables|Default|GetTextStrat) false false))))))))))

(event Custom|UISetPlayer1PReadyText
  ;[1 1 1] 플레이어 레디 텍스트 표시
  (Rendering|SetVisibility (Variables|Default|GetTextPlayer1PReady) true false))

(event Custom|UISetPlayer2PReadyText
  ;[1 1 1] 플레이어 레디 텍스트 표시
  (Rendering|SetVisibility (Variables|Default|GetTextPlayer2PReady) true false))

(event EventBeginPlay
  ;[1 1 1] 생명 아이콘 초기 생성, 생명 변수와 아이콘들을 변수에 저장
  (Utilities|FlowControl|Sequence
    (:then_0
      (bind _asthird_person_game_mode (Utilities|Casting|CastToThirdPersonGameMode (Game|GetGameMode)))
      (for _index (range 0 (- (Variables|/Game/Blueprints/Player/ThirdPersonGameMode.ThirdPersonGameMode_C|GetPlayer1PLife _asthird_person_game_mode) 1))
        (bind _returnvalue (AddComponent|AddStaticMeshComponent false (Math|Transform|MakeTransform (Math|Vector|MakeVector 3.3e+02 (Variables|Default|GetPlayer1PLifeIconPosY) -1.3e+02) "0, 0, 0" "0.200000,0.200000,0.200000")))
        (Variables|Default|SetPlayer1PLifeIconPosY (+ (Variables|Default|GetPlayer1PLifeIconPosY) -4e+01))
        (Utilities|Array|SetArrayElem (Variables|Default|GetPlayer1PLifeIconArr) _index _returnvalue true)))
    (:then_1
      (for _index_2 (range 0 (- (Variables|/Game/Blueprints/Player/ThirdPersonGameMode.ThirdPersonGameMode_C|GetPlayer2PLife _asthird_person_game_mode) 1))
        (bind _returnvalue_2 (AddComponent|AddStaticMeshComponent false (Math|Transform|MakeTransform (Math|Vector|MakeVector 3.3e+02 (Variables|Default|GetPlayer2PLifeIconPosY) -1.3e+02) "0, 0, 0" "0.200000,0.200000,0.200000")))
        (Variables|Default|SetPlayer2PLifeIconPosY (+ (Variables|Default|GetPlayer2PLifeIconPosY) 4e+01))
        (Utilities|Array|SetArrayElem (Variables|Default|GetPlayer2PLifeIconArr) _index_2 _returnvalue_2 true)))
    (:then_2
      (Collision|SetCollisionResponsetoAllChannels (Variables|Default|GetTextRestartButton) "ECR_Ignore"))))

(event Collision|EventActorBeginOverlap
  (params (OtherActor :type Actor%20Object%20Reference)))

(event EventTick
  (params (DeltaSeconds :type Float%20%28single-precision%29)))

(fn ConstructionScript)