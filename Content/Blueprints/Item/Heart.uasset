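; Heart pickup that grants an extra life to whichever of the two players touches it, then destroys itself.
; The construction script caches the actors tagged Player as Player1 or Player2, using the Player1P tag to tell them apart.
; On overlap, the same tags choose LifeUp1P or LifeUp2P on ThirdPersonGameMode, gated by casts on the cached player references.
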(event OnComponentBeginOverlap(Heart)
  (params (OverlappedComponent :type Primitive%20Component%20Object%20Reference) (OtherActor :type Actor%20Object%20Reference) (OtherComp :type Primitive%20Component%20Object%20Reference) (OtherBodyIndex :type Integer) (bFromSweep :type Boolean) (SweepResult :type Hit%20Result%20Structure%20%28by%20ref%29))
  (bind _returnvalue (Game|GetGameMode))
  ;[1 1 1] 먹으면 먹은 플레이어 LifeUp이벤트 실행
  (if (Actor|ActorHasTag OtherActor "Player")
    (if (Actor|ActorHasTag OtherActor "Player1P")
      (Utilities|Casting|CastToPlayer1P (Variables|Default|GetPlayer1))
      (bind _asthird_person_game_mode (Utilities|Casting|CastToThirdPersonGameMode _returnvalue))
      (Default|LifeUp1P _asthird_person_game_mode)
      (else
        (Utilities|Casting|CastToPlayer2P (Variables|Default|GetPlayer2))
        (bind _asthird_person_game_mode_2 (Utilities|Casting|CastToThirdPersonGameMode _returnvalue))
        (Default|LifeUp2P _asthird_person_game_mode_2)))
    (Actor|DestroyActor)))

(fn ConstructionScript
  (bind _outactors (Actor|GetAllActorswithTag "Player"))
  (for _array_element _outactors
    (if (Actor|ActorHasTag _array_element "Player1P")
      (Variables|Default|SetPlayer1 _array_element)
      (else
        (Variables|Default|SetPlayer2 _array_element)))))