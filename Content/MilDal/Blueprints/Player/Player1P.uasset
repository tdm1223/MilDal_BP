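; Player-one Character Blueprint with timed status effects and a respawn hold.
; Events toggle Reverse, Fast, InfiniteJump and SuperJump flags around delays, with the jump effects also changing jump count or hold time and super jump lasting a random time.
; Other events spawn a WInd actor at the character or briefly zero gravity and velocity for respawn.
; The construction script sets walk speed, air control, jump velocity and gravity.
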(event Custom|setSuperJump1P
  (bind _returnvalue (Math|Random|RandomIntegerinRange 1 5))
  (Variables|Default|SetSuperJump (not (Variables|Default|GetSuperJump)))
  (Variables|Default|SetJumpMaxHoldTime 5.0)
  (Development|PrintString (Utilities|String|ToString(Integer) _returnvalue))
  (Utilities|FlowControl|Delay (Math|Conversions|ToFloat(Integer) _returnvalue))
  (Variables|Default|SetSuperJump (not (Variables|Default|GetSuperJump)))
  (Variables|Default|SetJumpMaxHoldTime 0.0))

(event Custom|setInfiniteJump1P
  (Variables|Default|SetInfiniteJump (not (Variables|Default|GetInfiniteJump)))
  (Variables|Default|SetJumpMaxCount 100)
  (Utilities|FlowControl|Delay 5.0)
  (Variables|Default|SetInfiniteJump (not (Variables|Default|GetInfiniteJump)))
  (Variables|Default|SetJumpMaxCount 1))

(event Custom|MakeWind1P
  (Game|SpawnActorfromClass "/Game/MilDal/Blueprints/Item/WInd.WInd_C" (Transformation|GetActorTransform) "Undefined" 0 0))

(event Custom|setFast1P
  (Variables|Default|SetFast (not (Variables|Default|GetFast)))
  (Utilities|FlowControl|Delay 1.0)
  (Variables|Default|SetFast (not (Variables|Default|GetFast))))

(event Custom|setReverse1P
  (Variables|Default|SetReverse (not (Variables|Default|GetReverse)))
  (Utilities|FlowControl|Delay 5.0)
  (Variables|Default|SetReverse (not (Variables|Default|GetReverse))))

(event Custom|RespawnReady1P
  (bind _charactermovement (Variables|Character|GetCharacterMovement))
  ;[1 1 1] 리스폰을 대기하는 이벤트
  (Variables|/Script/Engine.CharacterMovementComponent|SetGravityScale _charactermovement 0.0)
  (Variables|/Script/Engine.MovementComponent|SetVelocity _charactermovement "0, 0, 0")
  (Utilities|FlowControl|Delay 2.0)
  (Variables|/Script/Engine.CharacterMovementComponent|SetGravityScale _charactermovement 2.0))

(fn ConstructionScript
  (bind _charactermovement (Variables|Character|GetCharacterMovement))
  ;[1 1 1] 캐릭터 최대 속도 세팅
  (Variables|/Script/Engine.CharacterMovementComponent|SetMaxWalkSpeed _charactermovement 1.2e+03)
  (Variables|/Script/Engine.CharacterMovementComponent|SetAirControl _charactermovement 1.0)
  (Variables|/Script/Engine.CharacterMovementComponent|SetJumpZVelocity _charactermovement 1.3e+03)
  (Variables|/Script/Engine.CharacterMovementComponent|SetGravityScale _charactermovement 2.0))