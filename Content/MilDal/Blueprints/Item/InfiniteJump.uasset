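; InfiniteJump is a pickup that grants infinite jump to whichever of the two players overlaps it, then destroys itself.
; The construction script finds actors tagged Player and caches them as Player1 or Player2 by the Player1P tag.
; On overlap, the same tag selects which cached player to cast and call SetInfiniteJump1P or SetInfiniteJump2P on, rather than using the overlapping actor directly.
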(event OnComponentBeginOverlap(InfiniteJump)
  (params (OverlappedComponent :type Primitive%20Component%20Object%20Reference) (OtherActor :type Actor%20Object%20Reference) (OtherComp :type Primitive%20Component%20Object%20Reference) (OtherBodyIndex :type Integer) (bFromSweep :type Boolean) (SweepResult :type Hit%20Result%20Structure%20%28by%20ref%29))
  (if (Actor|ActorHasTag OtherActor "Player")
    (if (Actor|ActorHasTag OtherActor "Player1P")
      (bind _asplayer_1p (Utilities|Casting|CastToPlayer1P (Variables|Default|GetPlayer1)))
      (Default|SetInfiniteJump1P _asplayer_1p)
      (else
        (bind _asplayer_2p (Utilities|Casting|CastToPlayer2P (Variables|Default|GetPlayer2)))
        (Default|SetInfiniteJump2P _asplayer_2p)))
    (Actor|DestroyActor)))

(fn ConstructionScript
  (bind _outactors (Actor|GetAllActorswithTag "Player"))
  (for _array_element _outactors
    (if (Actor|ActorHasTag _array_element "Player1P")
      (Variables|Default|SetPlayer1 _array_element)
      (else
        (Variables|Default|SetPlayer2 _array_element)))))