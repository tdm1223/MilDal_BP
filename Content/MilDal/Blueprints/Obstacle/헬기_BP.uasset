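; Helicopter obstacle Blueprint that flies along world Y while spinning its rotors.
; Each Tick offsets the Arrow component by a speed variable times DeltaSeconds, with Flag choosing positive or negative direction and no sweep.
; Main and rear rotors take fixed relative rotation steps per frame, independent of frame time.
; A DoOnce plays the helicopter sound a single time at the world origin, not at the helicopter.
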(event EventTick
  (params (DeltaSeconds :type Float%20%28single-precision%29))
  (bind _헬기이동속도 (Variables|Default|Get헬기이동속도))
  (bind _arrow (Variables|Default|GetArrow))
  (bind _returnvalue (* DeltaSeconds _헬기이동속도))
  ;[1 1 1] 헬기 날개회전
  ;[1 1 1] 헬기이동
  (if (Variables|Default|GetFlag)
    (Transformation|AddWorldOffset _arrow (Math|Vector|MakeVector 0.0 _returnvalue 0.0) false false)
    (else
      (Transformation|AddWorldOffset _arrow (Math|Vector|MakeVector 0.0 (* _returnvalue -1.0) 0.0) false false)))
  (Transformation|AddRelativeRotation (Variables|Default|Get헬기_main_rotor_parts02) "0,180.000000, 0" false false)
  (Transformation|AddRelativeRotation (Variables|Default|Get헬기_rear_rotor) "0, 0,100.000000" false false)
  (Utilities|FlowControl|DoOnce false
    (:Completed
      (Audio|PlaySoundatLocation "/Game/StaticMesh/Obstacle/헬기소리.헬기소리" "0, 0, 0"))))

(fn ConstructionScript)